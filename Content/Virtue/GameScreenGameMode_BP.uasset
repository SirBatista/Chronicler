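; Game mode for the game screen that makes sure an online session exists when play begins on the authority.
; It creates a BaseSessionServices task and, if no current session ID exists, stores a hard-coded local session name on the game instance.
; It then creates an advertised, joinable presence session through the online subsystem.
; Results print on screen, and a dedicated server quits if creation fails.
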(event `self.ReceiveBeginPlay`
  (`/Engine/EditorBlueprintResources/ActorMacros.Switch Has Authority`
    (:`Authority`
      (bind _instance (`/Game/ExampleOSS/Common/TaskLibraries/TaskLibraryActor.Create Task from Actor` "/Game/ExampleOSS/Common/BaseTasks/Session/BaseSessionServices.BaseSessionServices_C")
        (:`Return`
          (bind _output_get (set `self.Session Services` (cast `/Game/ExampleOSS/Common/BaseTasks/Session/BaseSessionServices` _instance :!pure true)))
          (bind _session_id (`/Game/ExampleOSS/Common/BaseTasks/Session/BaseSessionServices.Get Current Session Id` _output_get))
          (if (`KismetStringLibrary.EqualEqual_StrStr` _session_id)
            (set `/Game/ExampleOSS/Common/ExampleGameInstance.Joined Session Name` "MyLocalSessionName" (cast `/Game/ExampleOSS/Common/ExampleGameInstance` (`GameplayStatics.GetGameInstance`) :!pure true))
            (bind (_sessionname _bwassuccessful) (`OnlineSessionSubsystemCreateSession.CreateSession` (subsystem `OnlineSessionSubsystem`) (`OnlineIdentitySubsystem.GetUniquePlayerId` (subsystem `OnlineIdentitySubsystem`) 0) "MyLocalSessionName" (make `OnlineSessionSettingsBP` 0 0 true true false false false true true true false false))
              (:`OnCreateSessionComplete`
                (if _bwassuccessful
                  (`KismetSystemLibrary.PrintString` "Created a session!" true true (struct :`R` 0.089915 :`G` 1.0 :`A` 1.0) 10.0)
                  (else
                    (`KismetSystemLibrary.PrintString` "Failed to create session!")
                    (if (`KismetSystemLibrary.IsDedicatedServer`)
                      (`KismetSystemLibrary.PrintString` "Error: Dedicated server could not create session, so it is exiting" true true (struct :`R` 1.0 :`A` 1.0) 20.0)
                      (`KismetSystemLibrary.QuitGame` null "Quit" true))))))))))))

(fn `UserConstructionScript`)