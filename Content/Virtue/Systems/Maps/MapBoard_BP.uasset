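; Map board actor that displays a world map texture on a grid of tile meshes.
; RefreshTiles runs from the construction script, clearing TileHolder's children and rebuilding a TilesWide by TilesLong grid of MapBoardMesh_AC components centred on the holder.
; All tiles share one dynamic instance of MapBoardTop_MI in material slot 1, created when missing and fed WorldTexture as its Map parameter.
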(event `Refresh Tiles`
  (bind _returnvalue (`KismetMathLibrary.Max` (- (`self.Tiles Long`) 1)))
  (bind _returnvalue_2 (`KismetMathLibrary.Max` (- (`self.Tiles Wide`) 1)))
  (for _array_element (`SceneComponent.GetChildrenComponents` (`self.Tile Holder`) false)
    (`ActorComponent.K2_DestroyComponent` _array_element))
  (`/Engine/EditorBlueprintResources/StandardMacros.IsValid` (`self.Material Instance`)
    (:`Is Valid`
      _)
    (:`Is Not Valid`
      (bind _returnvalue_3 (`KismetMaterialLibrary.CreateDynamicMaterialInstance` "/Game/Virtue/Systems/Maps/MapBoardTop_MI.MapBoardTop_MI" "Board Top"))
      (set `self.Material Instance` _returnvalue_3)))
  (`MaterialInstanceDynamic.SetTextureParameterValue` (`self.Material Instance`) "Map" (`self.World Texture`))
  (for _index (range (+ _returnvalue_2 1))
    (for _index_2 (range (+ _returnvalue 1))
      (bind _returnvalue_4 (`|AddComponentByClass` "/Game/Virtue/Systems/Maps/MapBoardMesh_AC.MapBoardMesh_AC_C" false (`KismetMathLibrary.MakeTransform` (`KismetMathLibrary.MakeVector` (- (* _index 200.0) (* _returnvalue_2 100.0)) (- (* _index_2 200.0) (* _returnvalue 100.0))))))
      (`PrimitiveComponent.SetMaterial` _returnvalue_4 1 (`self.Material Instance`))
      (`SceneComponent.K2_AttachToComponent` _returnvalue_4 (`self.Tile Holder`) "None" "KeepRelative" "KeepRelative" "KeepRelative" true))))

(fn `UserConstructionScript`
  (`self.Refresh Tiles`))